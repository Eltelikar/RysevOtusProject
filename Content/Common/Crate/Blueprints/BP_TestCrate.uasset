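; Test interactable military crate that opens and closes its lid to show or hide a container inventory.
; A trigger box shows a text prompt and gates the Interact event, with Open and Finished flags tracking state and blocking input mid-animation.
; Timelines rotate the lid, play alongside audio on interaction, and toggle BPContainerComponent's inventory.
; After opening, AutoClose polls the container window and shuts the lid once it is no longer valid.
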(event `self.TriggerBox.OnComponentBeginOverlap`
  (params (OverlappedComponent :type "PrimitiveComponent Object Reference") (OtherActor :type "Actor Object Reference") (OtherComp :type "PrimitiveComponent Object Reference") (OtherBodyIndex :type Integer) (bFromSweep :type Boolean) (SweepResult :type "HitResult Structure (by ref)"))
  (set `self.InTriggerBox` true)
  (bind _returnvalue (`AddComponent|NODE_AddTextRenderComponent-0`))
  (`TextRenderComponent.K2_SetText` _returnvalue "Press \"E\" to open crate")
  (`TextRenderComponent.SetHorizontalAlignment` _returnvalue "EHTA_Center")
  (`TextRenderComponent.SetVerticalAlignment` _returnvalue "EVRTA_TextTop"))

(event `self.TriggerBox.OnComponentEndOverlap`
  (params (OverlappedComponent :type "PrimitiveComponent Object Reference") (OtherActor :type "Actor Object Reference") (OtherComp :type "PrimitiveComponent Object Reference") (OtherBodyIndex :type Integer))
  (set `self.InTriggerBox` false)
  (`TextRenderComponent.K2_SetText` (stale `self.TriggerBox.OnComponentBeginOverlap` _returnvalue) ""))

(event `/Game/ThirdPerson/Components/InventoryComponent/BPI_Interact.Interact`
  (params (Inventory :type "/Game/ThirdPerson/Components/InventoryComponent/BPC_Inventory Object Reference") (Player :type "PlayerController Object Reference") (InputAction :type "InputAction Object Reference"))
  (bind _sm_militarycratetop_05 (`self.SM_MilitaryCrateTop_05`))
  (set `self.Player` Player)
  (set `self.Input Action` InputAction)
  (if (`self.InTriggerBox`)
    (if (`self.Finished`)
      (set `self.Finished` false)
      (if (`self.Open`)
        (set `self.Open` false)
        (if (!= (`self.Input Action`) "/Game/ThirdPerson/Input/Actions/IA_LeftMouseAttack.IA_LeftMouseAttack")
          (`AddComponent|NODE_AddAudioComponent-0`)
          (bind (_direction _newtrack_0) (`Timeline|Timeline_0` :!via `PlayFromStart`)
            (:`Update`
              (`SceneComponent.K2_SetRelativeRotation` _sm_militarycratetop_05 (`KismetMathLibrary.MakeRotator` (* _newtrack_0 -1.0)) false false))
            (:`Finished`
              (set `self.Finished` true)
              (`KismetSystemLibrary.PrintString` "Crate has been closed")
              (`/Game/HUD/ContainerInventory/BP_ContainerComponent.ToggleContainerInventory` (`self.BP_ContainerComponent`) null))))
        (else
          (set `self.Open` true)
          (`AddComponent|NODE_AddAudioComponent-1`)
          (bind (_direction_2 _newtrack_0_2) (`Timeline|Timeline` :!via `PlayFromStart`)
            (:`Update`
              (`SceneComponent.K2_SetRelativeRotation` _sm_militarycratetop_05 (`KismetMathLibrary.MakeRotator` (* _newtrack_0_2 -1.0)) false false))
            (:`NewTrack_4`
              (set `self.Finished` true)
              (`KismetSystemLibrary.PrintString` "Crate has been opened")
              (`/Game/HUD/ContainerInventory/BP_ContainerComponent.ToggleContainerInventory` (`self.BP_ContainerComponent`) null)
              (`self.AutoClose`))))))))

(event `AutoClose`
  (`/Engine/EditorBlueprintResources/StandardMacros.IsValid` (`/Game/HUD/ContainerInventory/BP_ContainerComponent.UI_ContainerWindow` (`self.BP_ContainerComponent`)) :!label _label
    (:`Is Valid`
      (`KismetSystemLibrary.Delay` 0.2)
      (goto _label))
    (:`Is Not Valid`
      (if (`self.Finished`)
        (set `self.Finished` false)
        (if (`self.Open`)
          (bind (_direction _newtrack_0) (`Timeline|Timeline_1` :!via `PlayFromStart`)
            (:`Update`
              (`SceneComponent.K2_SetRelativeRotation` (`self.SM_MilitaryCrateTop_05`) (`KismetMathLibrary.MakeRotator` (* _newtrack_0 -1.0)) false false)
              (set `self.Open` false))
            (:`Finished`
              (set `self.Finished` true))))))))

(fn `UserConstructionScript`)