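; Player controller for the main menu that sets up menu input and restores saved audio volumes.
; On BeginPlay it toggles the menu widget through the game instance, shows the cursor and focuses that widget in Game and UI mode.
; It pushes a sound mix and applies BP_SaveAudio volumes as interface, music, SFX and voice class overrides.
; Without a save, it loops on a short delay back to the branch, without repeating the existence check.
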(event `self.ReceiveBeginPlay`
  (`GameplayStatics.PushSoundMixModifier` "/Game/Sounds/S_SoundMix.S_SoundMix")
  (message `/Game/HUD/MainMenu/BPInterface_MainMenu.ToggleMainMenu` (`GameplayStatics.GetGameInstance`))
  (set `self.bShowMouseCursor` true)
  (`WidgetBlueprintLibrary.SetInputMode_GameAndUIEx` self (`self.GetMainMenuWidget`))
  (bind _returnvalue (`GameplayStatics.DoesSaveGameExist` "BP_SaveAudio"))
  (if _returnvalue :!label _label
    (bind _returnvalue_2 (`GameplayStatics.LoadGameFromSlot` "BP_SaveAudio"))
    (bind _asbp_save_audio (cast `/Game/SettingSaves/BP_SaveAudio` _returnvalue_2))
    (bind _output_get (set `self.As BP Save Audio` _asbp_save_audio))
    (`|ExecutionSequence`
      (:`then_0`
        (`GameplayStatics.SetSoundMixClassOverride` "/Game/Sounds/S_SoundMix.S_SoundMix" "/Game/Sounds/S_Class_Interface.S_Class_Interface" (`/Game/SettingSaves/BP_SaveAudio.Interface_Volume` _output_get) 1.0 0.0))
      (:`then_1`
        (`GameplayStatics.SetSoundMixClassOverride` "/Game/Sounds/S_SoundMix.S_SoundMix" "/Game/Sounds/S_Class_Music.S_Class_Music" (`/Game/SettingSaves/BP_SaveAudio.Music_Volume` _output_get) 1.0 0.0))
      (:`then_2`
        (`GameplayStatics.SetSoundMixClassOverride` "/Game/Sounds/S_SoundMix.S_SoundMix" "/Game/Sounds/S_Class_SFX.S_Class_SFX" (`/Game/SettingSaves/BP_SaveAudio.SFX_Volume` _output_get) 1.0 0.0))
      (:`then_3`
        (`GameplayStatics.SetSoundMixClassOverride` "/Game/Sounds/S_SoundMix.S_SoundMix" "/Game/Sounds/S_Class_Voice.S_Class_Voice" (`/Game/SettingSaves/BP_SaveAudio.Voice_Volume` _output_get) 1.0 0.0)))
    (else
      (`KismetSystemLibrary.Delay` 0.2)
      (goto _label))))

(fn `GetMainMenuWidget`
  (returns (MainMenu :type "/Game/HUD/MainMenu/UI_Widgets/UI_MainMenu Object Reference"))
  (bind _mainmenu (message `/Game/HUD/MainMenu/BPInterface_MainMenu.GetReferenceMainMenu` (`GameplayStatics.GetGameInstance`)))
  (return _mainmenu))

(fn `UserConstructionScript`)