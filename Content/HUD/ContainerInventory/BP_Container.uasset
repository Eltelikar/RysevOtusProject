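; BP_Container is a world container with its own inventory of item objects.
; On BeginPlay it fills ContainerInventoryArray with InventorySize newly constructed BP_BaseItemObject instances.
; OpenContainerInventory creates a UI_ContainerSlot widget per entry, passing item and index, but does not attach them to a parent.
; Unconnected leftover nodes would create and show UI_ContainerWindow with cursor and Game-and-UI input, but never run.
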(event `self.ReceiveBeginPlay`
  (for _ (range (`self.InventorySize`))
    (bind _returnvalue (`|GenericCreateObject` "/Game/ThirdPerson/Components/InventoryComponent/BP_BaseItemObject.BP_BaseItemObject_C" null null null "" "" 0 0 0 "NewEnumerator10" "NewEnumerator0" "NewEnumerator0" null))
    (`KismetArrayLibrary.Array_AddUnique` (`self.ContainerInventoryArray`) _returnvalue)))

(fn `OpenContainerInventory`
  (params (PlayerController :type "PlayerController Object Reference (by ref)"))
  (for (_array_element _array_index) (`self.ContainerInventoryArray`)
    (`|CreateWidget` "/Game/HUD/ContainerInventory/UI_ContainerSlot.UI_ContainerSlot_C" null _array_element _array_index)))

(fn `UserConstructionScript`)