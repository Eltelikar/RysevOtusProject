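; Container inventory component that holds a container's item objects and shows or hides its window.
; On BeginPlay it fills ContainerInventory with newly constructed BP_BaseItemObject instances, one per InventorySize slot.
; ToggleContainerInventory either removes the open window or toggles the player's inventory and creates a UI_ContainerWindow bound to this component.
; Each toggle plays a sound and switches cursor visibility and input mode between game-only and game-and-UI.
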(event `self.ReceiveBeginPlay`
  (for _ (range (`self.InventorySize`))
    (bind _returnvalue (`|GenericCreateObject` "/Game/ThirdPerson/Components/InventoryComponent/BP_BaseItemObject.BP_BaseItemObject_C" null null null "" "" 0 0 0 "NewEnumerator10" "NewEnumerator0" "NewEnumerator0" null))
    (`KismetArrayLibrary.Array_AddUnique` (`self.ContainerInventory`) _returnvalue)))

(fn `ToggleContainerInventory`
  (params (PlayerController :type "PlayerController Object Reference"))
  (bind _returnvalue (`GameplayStatics.GetPlayerController` 0))
  (bind _returnvalue_2 (`GameplayStatics.GetPlayerController` 0))
  (bind _as_third_person_character (`self.As Third Person Character`))
  (bind _ui_containerwindow (`self.UI_ContainerWindow`)
    (:`then`
      (`GameplayStatics.PlaySound2D` "/Game/Sounds/INV_OPEN.INV_OPEN" 1.0 1.0 0.0 null _as_third_person_character)
      (`Widget.RemoveFromParent` _ui_containerwindow)
      (set `PlayerController.bShowMouseCursor` false _returnvalue)
      (`WidgetBlueprintLibrary.SetInputMode_GameOnly` _returnvalue)
      (set `self.UI_ContainerWindow` null))
    (:`else`
      (`GameplayStatics.PlaySound2D` "/Game/Sounds/INV_CLOSE.INV_CLOSE" 1.0 1.0 0.0 null _as_third_person_character)
      (bind _bpc_inventory (`/Game/ThirdPerson/Components/InventoryComponent/BPL_Inventory.BPC_InventoryReference`))
      (`/Game/ThirdPerson/Components/InventoryComponent/BPC_Inventory.Toggle Inentory` _bpc_inventory)
      (bind _returnvalue_3 (`|CreateWidget` "/Game/HUD/ContainerInventory/UI_ContainerWindow.UI_ContainerWindow_C" null self))
      (bind _output_get (set `self.UI_ContainerWindow` _returnvalue_3))
      (`UserWidget.AddToViewport` _output_get 0)
      (set `PlayerController.bShowMouseCursor` true _returnvalue_2)
      (`WidgetBlueprintLibrary.SetInputMode_GameAndUIEx` _returnvalue_2 (`self.UI_ContainerWindow`)))))