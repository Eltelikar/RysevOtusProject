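; BP_SaveSlots holds the list of save slot records for the main menu's saves menu.
; It exposes getters for that list and for a reference to itself.
; SetGameSaveSlot rejects a slot whose name already has a save game for user index 0, otherwise adds it uniquely and reports success.
; It only updates the array and does not write any save itself.
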(fn `GetSaveSlot`
  (returns (SaveGame :type "Array of /Game/HUD/MainMenu/UI_Widgets/SavesMenu/S_SaveGameSlotInfo Structure"))
  (return (`self.AllSlots`)))

(fn `SaveGameReference`
  (returns (Reference :type "/Game/HUD/MainMenu/UI_Widgets/SavesMenu/BP_SaveSlots Object Reference"))
  (return self))

(fn `SetGameSaveSlot`
  (params (SlotInfo :type "/Game/HUD/MainMenu/UI_Widgets/SavesMenu/S_SaveGameSlotInfo Structure"))
  (returns (`IsSave?` :type Boolean))
  (bind _returnvalue (`GameplayStatics.DoesSaveGameExist` SlotInfo_SlotName_2_313D9222446A87D93B5DED8D687D4425))
  (if _returnvalue
    (return false)
    (else
      (`KismetArrayLibrary.Array_AddUnique` (`self.AllSlots`) (`local.SlotInfo`))
      (return true))))